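; BP_Cannon is a one-shot cannon that damages BP_BOSS after the player holds F inside its trigger box.
; Box overlap arms it and shows a damage label and Console_Dialog hint.
; Tick polls the key, displays charge progress and resets on release, with damage and hold time both scaling from the mesh's X scale.
; Firing locks it, hides the UI and plays a timeline that offsets the player camera's Y position as a shake.
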(event OnComponentBeginOverlap(Box)
  (params (OverlappedComponent :type Primitive%20Component%20Object%20Reference) (OtherActor :type Actor%20Object%20Reference) (OtherComp :type Primitive%20Component%20Object%20Reference) (OtherBodyIndex :type Integer) (bFromSweep :type Boolean) (SweepResult :type Hit%20Result%20Structure%20%28by%20ref%29))
  (Utilities|Casting|CastToBP_ThirdPersonCharacter OtherActor)
  (if (Variables|Default|GetOnce)
    (Variables|Default|SetAble true)
    (Rendering|SetVisibility (Variables|Default|GetTextRender) true false)
    (bind _returnvalue (Actor|GetActorOfClass "/Game/Resources/BP/Console/Console_Dialog.Console_Dialog_C"))
    (Default|SendHint _returnvalue "<System>按住F开炮</>")))

(event OnComponentEndOverlap(Box)
  (params (OverlappedComponent :type Primitive%20Component%20Object%20Reference) (OtherActor :type Actor%20Object%20Reference) (OtherComp :type Primitive%20Component%20Object%20Reference) (OtherBodyIndex :type Integer))
  (Utilities|Casting|CastToBP_ThirdPersonCharacter OtherActor)
  (if (Variables|Default|GetOnce)
    (Variables|Default|SetAble false)
    (Rendering|SetVisibility (Variables|Default|GetTextRender) false false)
    (bind _returnvalue (Actor|GetActorOfClass "/Game/Resources/BP/Console/Console_Dialog.Console_Dialog_C"))
    (Default|SendHint _returnvalue)))

(event EventBeginPlay
  (Variables|Default|SetisHolding false)
  (Variables|Default|SetTime 0.0)
  (Variables|Default|SetOnce true)
  (Variables|Default|SetAble false)
  (Rendering|SetVisibility (Variables|Default|GetTextRender) false false)
  (Input|EnableInput (Game|GetPlayerController 0))
  (Rendering|SetVisibility (Variables|Default|GetTextRender1) false false))

(event Collision|EventActorBeginOverlap
  (params (OtherActor :type Actor%20Object%20Reference)))

(event EventTick
  (params (DeltaSeconds :type Float%20%28single-precision%29))
  (bind _staticmesh (Variables|Default|GetStaticMesh))
  (bind _returnvalue (Transformation|GetWorldScale _staticmesh))
  (bind _returnvalue_2 (* (.x _returnvalue) 1e+02))
  (bind _returnvalue_3 (Actor|GetActorOfClass "/Game/Resources/BP/BP/Parent/BP_BOSS.BP_BOSS_C"))
  (if (Utilities|IsValid _returnvalue_3)
    (if (Variables|Default|GetOnce)
      (Rendering|Components|TextRender|SetText (Variables|Default|GetTextRender) (Utilities|Text|ToText(String) (Utilities|String|Append (Utilities|String|ToString(Text) (Utilities|Text|ToText(Float) _returnvalue_2 "HalfToEven")) "Damage")))
      (Variables|Default|SetTargetTime (* (.x _returnvalue) 3.0))
      (if (Variables|Default|GetAble)
        (if (Game|Player|IsInputKeyDown (Game|GetPlayerController 0) "F")
          (Rendering|SetVisibility (Variables|Default|GetTextRender1) true false)
          (Variables|Default|SetTime (+ (Variables|Default|GetTime) DeltaSeconds))
          (Rendering|Components|TextRender|SetText (Variables|Default|GetTextRender1) (Utilities|Text|ToText(Float) (/ (Variables|Default|GetTime) (Variables|Default|GetTargetTime)) "HalfToEven"))
          (if (>= (Variables|Default|GetTime) (Variables|Default|GetTargetTime))
            (Variables|Default|SetOnce false)
            (bind _returnvalue_4 (Actor|GetActorOfClass "/Game/Resources/BP/BP/Parent/BP_BOSS.BP_BOSS_C"))
            (Default|Damage _returnvalue_4 _returnvalue_2)
            (Rendering|SetVisibility (Variables|Default|GetTextRender) false false)
            (Rendering|SetVisibility (Variables|Default|GetTextRender1) false false)
            (bind _returnvalue_5 (Actor|GetActorOfClass "/Game/Resources/BP/Console/Console_Dialog.Console_Dialog_C"))
            (Default|SendHint _returnvalue_5)
            (bind _新建轨道_0 (Timeline|时间轴 Play)
              (:Update
                (Transformation|SetRelativeLocation (Actor|GetComponentbyClass (Game|GetPlayerCharacter 0) "/Script/Engine.CameraComponent") (Math|Vector|MakeVector 0.0 (+ (* _新建轨道_0 3.0) 5e+01) 0.0) false false)
                (Utilities|FlowControl|Delay 1.0)
                (Timeline|时间轴 Stop))))
          (else
            (Rendering|SetVisibility (Variables|Default|GetTextRender1) false false)
            (Variables|Default|SetTime 0.0)))))))

(fn ConstructionScript)