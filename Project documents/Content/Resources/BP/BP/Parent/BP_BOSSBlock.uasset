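; BP_BOSSBlock is a trigger, likely for a boss area, that reveals a hidden block when the player character walks in.
; The referenced Block's root is hidden on BeginPlay and shown when BP_ThirdPersonCharacter overlaps the Box.
; If the Destroy reference is valid, it destroys that actor and plays a timeline offsetting the player camera's relative Y location.
; A half-second Delay on the timeline's update stops the camera motion.
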(event OnComponentBeginOverlap(Box)
  (params (OverlappedComponent :type Primitive%20Component%20Object%20Reference) (OtherActor :type Actor%20Object%20Reference) (OtherComp :type Primitive%20Component%20Object%20Reference) (OtherBodyIndex :type Integer) (bFromSweep :type Boolean) (SweepResult :type Hit%20Result%20Structure%20%28by%20ref%29))
  (bind _destroy (Variables|Default|GetDestroy))
  (Utilities|Casting|CastToBP_ThirdPersonCharacter OtherActor)
  (Rendering|SetVisibility (Variables|/Script/Engine.Actor|GetRootComponent (Variables|Default|GetBlock)) true false)
  (if (Utilities|IsValid _destroy)
    (Actor|DestroyActor _destroy)
    (bind _新建轨道_0 (Timeline|时间轴 Play)
      (:Update
        (Transformation|SetRelativeLocation (Actor|GetComponentbyClass (Game|GetPlayerCharacter 0) "/Script/Engine.CameraComponent") (Math|Vector|MakeVector 0.0 (+ (* _新建轨道_0 3.0) 5e+01) 0.0) false false)
        (Utilities|FlowControl|Delay 0.5)
        (Timeline|时间轴 Stop)))))

(event EventBeginPlay
  (Rendering|SetVisibility (Variables|/Script/Engine.Actor|GetRootComponent (Variables|Default|GetBlock)) false false))

(event Collision|EventActorBeginOverlap
  (params (OtherActor :type Actor%20Object%20Reference)))

(event EventTick
  (params (DeltaSeconds :type Float%20%28single-precision%29)))

(fn ConstructionScript)