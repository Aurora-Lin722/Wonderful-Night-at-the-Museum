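; BP_Plate is a trigger plate that slides two target actors open while something overlaps its Box and back when the overlap ends.
; On BeginPlay it caches each target's start location and an end point offset against that actor's right vector.
; Overlap events set the Open flag and Light status, then play or reverse a Timeline from its current position to lerp both targets.
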(event OnComponentBeginOverlap(Box)
  (params (OverlappedComponent :type Primitive%20Component%20Object%20Reference) (OtherActor :type Actor%20Object%20Reference) (OtherComp :type Primitive%20Component%20Object%20Reference) (OtherBodyIndex :type Integer) (bFromSweep :type Boolean) (SweepResult :type Hit%20Result%20Structure%20%28by%20ref%29))
  (Variables|Default|SetOpen true)
  (CallFunction|Stop)
  (CallFunction|Start)
  (Variables|/Game/Resources/BP/BP/Parent/BP_IndicatorLight.BP_IndicatorLight_C|Setstatus (Variables|Default|GetLight) true))

(event OnComponentEndOverlap(Box)
  (params (OverlappedComponent :type Primitive%20Component%20Object%20Reference) (OtherActor :type Actor%20Object%20Reference) (OtherComp :type Primitive%20Component%20Object%20Reference) (OtherBodyIndex :type Integer))
  (Variables|Default|SetOpen false)
  (CallFunction|Stop)
  (CallFunction|Reverse)
  (Variables|/Game/Resources/BP/BP/Parent/BP_IndicatorLight.BP_IndicatorLight_C|Setstatus (Variables|Default|GetLight) false))

(event Custom|Reverse
  (bind _新建轨道_0 (Timeline|时间轴 Reverse)
    (:Update
      (Variables|Default|SetCurrentTime _新建轨道_0)
      (Transformation|SetActorLocation (Variables|Default|GetTarget1) (Math|Vector|Lerp(Vector) (Variables|Default|GetStartVec1) (Variables|Default|GetEndVec1) _新建轨道_0) false false)
      (Transformation|SetActorLocation (Variables|Default|GetTarget2) (Math|Vector|Lerp(Vector) (Variables|Default|GetStartVec1_0) (Variables|Default|GetEndVec1_0) _新建轨道_0) false false))))

(event Custom|Start
  (bind _新建轨道_0 (Timeline|时间轴 Play)
    (:Update
      (Variables|Default|SetCurrentTime _新建轨道_0)
      (Transformation|SetActorLocation (Variables|Default|GetTarget1) (Math|Vector|Lerp(Vector) (Variables|Default|GetStartVec1) (Variables|Default|GetEndVec1) _新建轨道_0) false false)
      (Transformation|SetActorLocation (Variables|Default|GetTarget2) (Math|Vector|Lerp(Vector) (Variables|Default|GetStartVec1_0) (Variables|Default|GetEndVec1_0) _新建轨道_0) false false))))

(event Custom|Stop
  (bind _新建轨道_0 (Timeline|时间轴 Stop)
    (:Update
      (Variables|Default|SetCurrentTime _新建轨道_0)
      (Transformation|SetActorLocation (Variables|Default|GetTarget1) (Math|Vector|Lerp(Vector) (Variables|Default|GetStartVec1) (Variables|Default|GetEndVec1) _新建轨道_0) false false)
      (Transformation|SetActorLocation (Variables|Default|GetTarget2) (Math|Vector|Lerp(Vector) (Variables|Default|GetStartVec1_0) (Variables|Default|GetEndVec1_0) _新建轨道_0) false false))))

(event EventBeginPlay
  (bind _target1 (Variables|Default|GetTarget1))
  (bind _target2 (Variables|Default|GetTarget2))
  (bind _returnvalue (Transformation|GetActorLocation _target2))
  (bind _returnvalue_2 (Transformation|GetActorLocation _target1))
  (Variables|Default|SetStartVec1 _returnvalue_2)
  (Variables|Default|SetEndVec1 (- _returnvalue_2 (* (Transformation|GetActorRightVector _target1) 1e+02)))
  (Variables|Default|SetStartVec1_0 _returnvalue)
  (Variables|Default|SetEndVec1_0 (- _returnvalue (* (Transformation|GetActorRightVector _target2) 1e+02))))

(event Collision|EventActorBeginOverlap
  (params (OtherActor :type Actor%20Object%20Reference)))

(event EventTick
  (params (DeltaSeconds :type Float%20%28single-precision%29)))

(fn ConstructionScript)