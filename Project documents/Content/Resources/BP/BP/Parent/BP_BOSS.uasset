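; BP_BOSS is a boss that moves vertically at a set speed and can be damaged until defeated.
; Generate places it at a fixed start, creates its health bar and starts movement; Damage subtracts from HP stored on that widget.
; At zero HP, Tick removes the bar, waits, calls Sequence23 and destroys the boss.
; Box overlap destroys cannons, or resets the boss, teleports the player and clears BP_BOSSTrigger's Exist flag.
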(event OnComponentBeginOverlap(Box)
  (params (OverlappedComponent :type Primitive%20Component%20Object%20Reference) (OtherActor :type Actor%20Object%20Reference) (OtherComp :type Primitive%20Component%20Object%20Reference) (OtherBodyIndex :type Integer) (bFromSweep :type Boolean) (SweepResult :type Hit%20Result%20Structure%20%28by%20ref%29))
  (bind _asbp_third_person_character (Utilities|Casting|CastToBP_ThirdPersonCharacter OtherActor)
    (:then
      (Variables|Default|SetMove false)
      (Widget|RemovefromParent (Variables|Default|GetWidGet))
      (Transformation|SetActorLocationAndRotation "-10620.000000,4820.000000,-900.000000" "0, 0, 0")
      (Transformation|Teleport _asbp_third_person_character "-9850.000000,4700.000000,450.000000" "0.000000,180.000000,0.000000")
      (bind _returnvalue (Actor|GetActorOfClass "/Game/Resources/BP/BP/Parent/BP_BOSSTrigger.BP_BOSSTrigger_C"))
      (Variables|/Game/Resources/BP/BP/Parent/BP_BOSSTrigger.BP_BOSSTrigger_C|SetExist _returnvalue false))
    (:CastFailed
      (bind _asbp_cannon (Utilities|Casting|CastToBP_Cannon OtherActor))
      (Actor|DestroyActor _asbp_cannon))))

(event EventBeginPlay
  (Variables|Default|SetMove false))

(event Collision|EventActorBeginOverlap
  (params (OtherActor :type Actor%20Object%20Reference)))

(event EventTick
  (params (DeltaSeconds :type Float%20%28single-precision%29))
  (bind _widget (Variables|Default|GetWidGet))
  (if (Variables|Default|GetMove)
    (Transformation|AddWorldOffset (Variables|Default|GetStaticMesh) (Math|Vector|MakeVector 0.0 0.0 (* (Variables|Default|GetSpeed) DeltaSeconds)) false false)
    (if (<= (Variables|/Game/Resources/BP/WBP/WBP_BossHP.WBP_BossHP_C|GetCurrentHP _widget) 0.0)
      (Widget|RemovefromParent _widget)
      (Utilities|FlowControl|Delay 1.5)
      (Default|CallSequence23)
      (Actor|DestroyActor))))

(event EventDamage
  (params (Damage :type Float%20%28double-precision%29))
  (bind _widget (Variables|Default|GetWidGet))
  (Variables|/Game/Resources/BP/WBP/WBP_BossHP.WBP_BossHP_C|SetCurrentHP _widget (- (Variables|/Game/Resources/BP/WBP/WBP_BossHP.WBP_BossHP_C|GetCurrentHP _widget) Damage)))

(event EventGenerate
  (Transformation|SetActorLocationAndRotation "-10620.000000,4820.000000,-900.000000" "0, 0, 0")
  (bind _returnvalue (UserInterface|CreateWidget "/Game/Resources/BP/WBP/WBP_BossHP.WBP_BossHP_C" (Game|GetPlayerController 0)))
  (bind _output_get (Variables|Default|SetWidGet _returnvalue))
  (UserInterface|Viewport|AddtoViewport _output_get 0)
  (Variables|/Game/Resources/BP/WBP/WBP_BossHP.WBP_BossHP_C|SetCurrentHP _output_get (Variables|/Game/Resources/BP/WBP/WBP_BossHP.WBP_BossHP_C|GetMaxHP _output_get))
  (Variables|Default|SetMove true))

(fn ConstructionScript)