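; BP_Cannon1 is a one-shot cannon interactable that the third-person character fires by holding F inside its Box trigger.
; Box overlaps arm it and show or clear a hint through Console_Dialog, while Tick accumulates hold time and displays progress on a TextRender, resetting on release.
; After a one-second hold it destroys the Aim actor, clears the hint and runs a timeline that briefly offsets the player camera's relative location.
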(event OnComponentBeginOverlap(Box)
  (params (OverlappedComponent :type Primitive%20Component%20Object%20Reference) (OtherActor :type Actor%20Object%20Reference) (OtherComp :type Primitive%20Component%20Object%20Reference) (OtherBodyIndex :type Integer) (bFromSweep :type Boolean) (SweepResult :type Hit%20Result%20Structure%20%28by%20ref%29))
  (Utilities|Casting|CastToBP_ThirdPersonCharacter OtherActor)
  (if (Variables|Default|GetOnce)
    (Variables|Default|SetAble true)
    (bind _returnvalue (Actor|GetActorOfClass "/Game/Resources/BP/Console/Console_Dialog.Console_Dialog_C"))
    (Default|SendHint _returnvalue "<System>按住F开炮</>")))

(event OnComponentEndOverlap(Box)
  (params (OverlappedComponent :type Primitive%20Component%20Object%20Reference) (OtherActor :type Actor%20Object%20Reference) (OtherComp :type Primitive%20Component%20Object%20Reference) (OtherBodyIndex :type Integer))
  (Utilities|Casting|CastToBP_ThirdPersonCharacter OtherActor)
  (if (Variables|Default|GetOnce)
    (Variables|Default|SetAble false)
    (bind _returnvalue (Actor|GetActorOfClass "/Game/Resources/BP/Console/Console_Dialog.Console_Dialog_C"))
    (Default|SendHint _returnvalue)))

(event EventBeginPlay
  (Variables|Default|SetisHolding false)
  (Variables|Default|SetTime 0.0)
  (Variables|Default|SetOnce true)
  (Variables|Default|SetAble false)
  (Input|EnableInput (Game|GetPlayerController 0))
  (Rendering|SetVisibility (Variables|Default|GetTextRender1) false false))

(event Collision|EventActorBeginOverlap
  (params (OtherActor :type Actor%20Object%20Reference)))

(event EventTick
  (params (DeltaSeconds :type Float%20%28single-precision%29))
  (if (Variables|Default|GetOnce)
    (Variables|Default|SetTargetTime 1.0)
    (if (Variables|Default|GetAble)
      (if (Game|Player|IsInputKeyDown (Game|GetPlayerController 0) "F")
        (Rendering|SetVisibility (Variables|Default|GetTextRender1) true false)
        (Variables|Default|SetTime (+ (Variables|Default|GetTime) DeltaSeconds))
        (Rendering|Components|TextRender|SetText (Variables|Default|GetTextRender1) (Utilities|Text|ToText(Float) (/ (Variables|Default|GetTime) (Variables|Default|GetTargetTime)) "HalfToEven"))
        (if (>= (Variables|Default|GetTime) (Variables|Default|GetTargetTime))
          (Variables|Default|SetOnce false)
          (Actor|DestroyActor (Variables|Default|GetAim))
          (Rendering|SetVisibility (Variables|Default|GetTextRender1) false false)
          (bind _returnvalue (Actor|GetActorOfClass "/Game/Resources/BP/Console/Console_Dialog.Console_Dialog_C"))
          (Default|SendHint _returnvalue)
          (bind _新建轨道_0 (Timeline|时间轴 Play)
            (:Update
              (Transformation|SetRelativeLocation (Actor|GetComponentbyClass (Game|GetPlayerCharacter 0) "/Script/Engine.CameraComponent") (Math|Vector|MakeVector 0.0 (+ (* _新建轨道_0 3.0) 5e+01) 0.0) false false)
              (Utilities|FlowControl|Delay 1.0)
              (Timeline|时间轴 Stop))))
        (else
          (Rendering|SetVisibility (Variables|Default|GetTextRender1) false false)
          (Variables|Default|SetTime 0.0))))))

(fn ConstructionScript)