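; BP_DialogTrigger is a trigger volume, kept in a Parent folder, that sends dialog when something overlaps its Box.
; An overlap while CanTrigger is set finds the Console_Dialog actor by class, passes it DialogQueue, then clears CanTrigger.
; Unless Once is set, Tick re-arms the trigger through a five-second Delay, so the dialog can repeat.
; The overlap does not filter which actor entered.
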(event OnComponentBeginOverlap(Box)
  (params (OverlappedComponent :type Primitive%20Component%20Object%20Reference) (OtherActor :type Actor%20Object%20Reference) (OtherComp :type Primitive%20Component%20Object%20Reference) (OtherBodyIndex :type Integer) (bFromSweep :type Boolean) (SweepResult :type Hit%20Result%20Structure%20%28by%20ref%29))
  (if (Variables|Default|GetCanTrigger)
    (bind _returnvalue (Actor|GetActorOfClass "/Game/Resources/BP/Console/Console_Dialog.Console_Dialog_C"))
    (bind _output_get (Variables|Default|SetDialogConsole _returnvalue))
    (Default|SendDialog _output_get (Variables|Default|GetDialogQueue))
    (Variables|Default|SetCanTrigger false)))

(event EventBeginPlay
  (Variables|Default|SetCanTrigger true))

(event Collision|EventActorBeginOverlap
  (params (OtherActor :type Actor%20Object%20Reference)))

(event EventTick
  (params (DeltaSeconds :type Float%20%28single-precision%29))
  (if (not (Variables|Default|GetOnce))
    (if (not (Variables|Default|GetCanTrigger))
      (Utilities|FlowControl|Delay 5.0)
      (Variables|Default|SetCanTrigger true))))

(fn ConstructionScript)