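; BP_IndicatorLight is an indicator light actor that shows a boolean Status with its Red and Green lights.
; Green is lit when Status is true and Red when it is false, with the other light set to zero intensity.
; BeginPlay sets the initial state, and Tick reapplies it every frame by polling Status rather than reacting to changes.
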(event EventBeginPlay
  (Rendering|Components|Light|SetIntensity (Variables|Default|GetRed) 0.0)
  (Rendering|Components|Light|SetIntensity (Variables|Default|GetGreen) 0.0)
  (if (Variables|Default|Getstatus)
    (Rendering|Components|Light|SetIntensity (Variables|Default|GetGreen) 5e+03)
    (else
      (Rendering|Components|Light|SetIntensity (Variables|Default|GetRed) 5e+03))))

(event Collision|EventActorBeginOverlap
  (params (OtherActor :type Actor%20Object%20Reference)))

(event EventTick
  (params (DeltaSeconds :type Float%20%28single-precision%29))
  (bind _red (Variables|Default|GetRed))
  (bind _green (Variables|Default|GetGreen))
  (if (Variables|Default|Getstatus)
    (Rendering|Components|Light|SetIntensity _green 5e+03)
    (Rendering|Components|Light|SetIntensity _red 0.0)
    (else
      (Rendering|Components|Light|SetIntensity _red 5e+03)
      (Rendering|Components|Light|SetIntensity _green 0.0))))

(fn ConstructionScript)