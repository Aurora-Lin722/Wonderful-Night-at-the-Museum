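; BP_DoorOpen is an interactive door that opens when the player character stands in its Box and presses F.
; Box overlaps toggle the Able flag and the Console_Dialog hint until Done is set.
; Tick polls F, sets the Light status and plays a timeline sliding two target actors against their right vectors, lerping from current location.
; Finishing sets Done and clears the hint, but leaves Able unchanged.
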(event OnComponentBeginOverlap(Box)
  (params (OverlappedComponent :type Primitive%20Component%20Object%20Reference) (OtherActor :type Actor%20Object%20Reference) (OtherComp :type Primitive%20Component%20Object%20Reference) (OtherBodyIndex :type Integer) (bFromSweep :type Boolean) (SweepResult :type Hit%20Result%20Structure%20%28by%20ref%29))
  (if (not (Variables|Default|GetDone?))
    (Utilities|Casting|CastToBP_ThirdPersonCharacter OtherActor)
    (bind _returnvalue (Actor|GetActorOfClass "/Game/Resources/BP/Console/Console_Dialog.Console_Dialog_C"))
    (bind _output_get (Variables|Default|SetConsoleDialog _returnvalue))
    (Default|SendHint _output_get (Variables|Default|GetHint))
    (Variables|Default|SetAble true)))

(event OnComponentEndOverlap(Box)
  (params (OverlappedComponent :type Primitive%20Component%20Object%20Reference) (OtherActor :type Actor%20Object%20Reference) (OtherComp :type Primitive%20Component%20Object%20Reference) (OtherBodyIndex :type Integer))
  (if (not (Variables|Default|GetDone?))
    (Utilities|Casting|CastToBP_ThirdPersonCharacter OtherActor)
    (Default|SendHint (Variables|Default|GetConsoleDialog))
    (Variables|Default|SetAble false)))

(event EventBeginPlay
  (Variables|Default|SetDone? false)
  (Variables|Default|SetAble false)
  (Input|EnableInput (Game|GetPlayerController 0)))

(event Collision|EventActorBeginOverlap
  (params (OtherActor :type Actor%20Object%20Reference)))

(event EventTick
  (params (DeltaSeconds :type Float%20%28single-precision%29))
  (bind _target1 (Variables|Default|GetTarget1))
  (bind _target2 (Variables|Default|GetTarget2))
  (bind _returnvalue (Transformation|GetActorLocation _target2))
  (bind _returnvalue_2 (Transformation|GetActorLocation _target1))
  (if (Variables|Default|GetAble)
    (if (Game|Player|IsInputKeyDown (Game|GetPlayerController 0) "F")
      (Variables|/Game/Resources/BP/BP/Parent/BP_IndicatorLight.BP_IndicatorLight_C|Setstatus (Variables|Default|GetLight) true)
      (bind _新建轨道_0 (Timeline|时间轴 PlayFromStart)
        (:Update
          (Transformation|SetActorLocation _target1 (Math|Vector|Lerp(Vector) _returnvalue_2 (- _returnvalue_2 (* (Transformation|GetActorRightVector _target1) 1e+02)) _新建轨道_0) false false)
          (Transformation|SetActorLocation _target2 (Math|Vector|Lerp(Vector) _returnvalue (- _returnvalue (* (Transformation|GetActorRightVector _target2) 1e+02)) _新建轨道_0) false false))
        (:Finished
          (Variables|Default|SetDone? true)
          (Default|SendHint (stale OnComponentBeginOverlap(Box) _output_get)))))))

(fn ConstructionScript)