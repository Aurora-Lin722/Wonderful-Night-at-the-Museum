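; BP_BOSSTrigger is a box trigger that lets the player start the boss encounter by pressing F.
; Overlap with the third-person character toggles a Console_Dialog hint and arms key polling on Tick.
; Pressing F calls CallSequence22, waits out a long delay, then calls Generate on BP_BOSS and destroys Target0.
; A timeline then shifts the player camera's lateral offset, and the Exist flag blocks retriggering.
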(event OnComponentBeginOverlap(Box)
  (params (OverlappedComponent :type Primitive%20Component%20Object%20Reference) (OtherActor :type Actor%20Object%20Reference) (OtherComp :type Primitive%20Component%20Object%20Reference) (OtherBodyIndex :type Integer) (bFromSweep :type Boolean) (SweepResult :type Hit%20Result%20Structure%20%28by%20ref%29))
  (Utilities|Casting|CastToBP_ThirdPersonCharacter OtherActor)
  (bind _returnvalue (Actor|GetActorOfClass "/Game/Resources/BP/Console/Console_Dialog.Console_Dialog_C"))
  (Default|SendHint _returnvalue "<System>F  启动</>")
  (Variables|Default|SetAble true))

(event OnComponentEndOverlap(Box)
  (params (OverlappedComponent :type Primitive%20Component%20Object%20Reference) (OtherActor :type Actor%20Object%20Reference) (OtherComp :type Primitive%20Component%20Object%20Reference) (OtherBodyIndex :type Integer))
  (Utilities|Casting|CastToBP_ThirdPersonCharacter OtherActor)
  (bind _returnvalue (Actor|GetActorOfClass "/Game/Resources/BP/Console/Console_Dialog.Console_Dialog_C"))
  (Default|SendHint _returnvalue)
  (Variables|Default|SetAble false))

(event EventBeginPlay
  (Variables|Default|SetAble false)
  (Input|EnableInput (Game|GetPlayerController 0)))

(event Collision|EventActorBeginOverlap
  (params (OtherActor :type Actor%20Object%20Reference)))

(event EventTick
  (params (DeltaSeconds :type Float%20%28single-precision%29))
  (if (Variables|Default|GetAble)
    (if (not (Variables|Default|GetExist))
      (if (Game|Player|IsInputKeyDown (Game|GetPlayerController 0) "F")
        (bind _returnvalue (Actor|GetActorOfClass "/Game/Resources/BP/BP/Parent/BP_BOSS.BP_BOSS_C"))
        (bind _returnvalue_2 (Actor|GetActorOfClass "/Game/Resources/BP/Console/Console_Dialog.Console_Dialog_C"))
        (Default|SendHint _returnvalue_2)
        (Default|CallSequence22)
        (Utilities|FlowControl|Delay 14.0)
        (Default|Generate _returnvalue)
        (Actor|DestroyActor (Variables|Default|GetTarget_0))
        (Variables|Default|SetAble false)
        (Variables|Default|SetExist true)
        (bind _新建轨道_0 (Timeline|时间轴 Play)
          (:Update
            (Transformation|SetRelativeLocation (Actor|GetComponentbyClass (Game|GetPlayerCharacter 0) "/Script/Engine.CameraComponent") (Math|Vector|MakeVector 0.0 (+ (* _新建轨道_0 3.0) 5e+01) 0.0) false false)
            (Utilities|FlowControl|Delay 2.0)
            (Timeline|时间轴 Stop)))))))

(fn ConstructionScript)